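; Player character Blueprint that drives the mesh animation from the character's current state.
; Every Tick it reads GetCharacterState and switches between normal, dodging and flying, playing Idle, Forward_Roll or Flying.
; PlayAnimation is called directly on the mesh every frame with looping off, with no transition logic in this graph.
; A debug print of the movement mode is left unconnected, and BeginPlay, overlap and construction are empty.
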(event EventBeginPlay)

(event Collision|EventActorBeginOverlap
  (params (OtherActor :type Actor%20Object%20Reference)))

(event EventTick
  (params (DeltaSeconds :type Float%20%28single-precision%29))
  (bind _returnvalue (Class|ACharacterBase|GetCharacterState))
  (switch Utilities|FlowControl|Switch|SwitchonESF_CharacterState _returnvalue
    (:Normal
      (Components|Animation|PlayAnimation (Variables|Character|GetMesh) "/Game/Models/Test/Animations/Idle.Idle" false))
    (:Avoid
      (Components|Animation|PlayAnimation (Variables|Character|GetMesh) "/Game/BP/Player/Anim/Forward_Roll.Forward_Roll" false))
    (:Fly
      (Components|Animation|PlayAnimation (Variables|Character|GetMesh) "/Game/BP/Player/Anim/Flying.Flying" false))))

(fn ConstructionScript)